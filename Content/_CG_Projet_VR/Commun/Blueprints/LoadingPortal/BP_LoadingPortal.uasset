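; BP_LoadingPortal is a portal trigger that streams sublevels in as a Character passes through it.
; On begin and end overlap, the dot product of 2D velocity direction and actor forward vector gives the crossing direction.
; Entering forward or exiting backward loads LoadSubLevel; the opposite crossings load UnloadSubLevel.
; Both levels load non-blocking and become visible; despite the UnloadSubLevel name, nothing is unloaded here.
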(event `self.Portal.OnComponentBeginOverlap`
  (params (OverlappedComponent :type "PrimitiveComponent Object Reference") (OtherActor :type "Actor Object Reference") (OtherComp :type "PrimitiveComponent Object Reference") (OtherBodyIndex :type Integer) (bFromSweep :type Boolean) (SweepResult :type "HitResult Structure (by ref)"))
  (bind _ascharacter (cast `Character` OtherActor))
  (if (> (`KismetMathLibrary.Dot_VectorVector` (`KismetMathLibrary.Vector_Normal2D` (`self.GetVelocity` _ascharacter)) (`self.GetActorForwardVector`)) 0.0)
    (`GameplayStatics.LoadStreamLevelBySoftObjectPtr` (`self.LoadSubLevel`) true)
    (else
      (`GameplayStatics.LoadStreamLevelBySoftObjectPtr` (`self.UnloadSubLevel`) true))))

(event `self.Portal.OnComponentEndOverlap`
  (params (OverlappedComponent :type "PrimitiveComponent Object Reference") (OtherActor :type "Actor Object Reference") (OtherComp :type "PrimitiveComponent Object Reference") (OtherBodyIndex :type Integer))
  (bind _ascharacter (cast `Character` OtherActor))
  (if (> (`KismetMathLibrary.Dot_VectorVector` (`KismetMathLibrary.Vector_Normal2D` (`self.GetVelocity` _ascharacter)) (`self.GetActorForwardVector`)) 0.0)
    (`GameplayStatics.LoadStreamLevelBySoftObjectPtr` (`self.UnloadSubLevel`) true)
    (else
      (`GameplayStatics.LoadStreamLevelBySoftObjectPtr` (`self.LoadSubLevel`) true))))

(fn `UserConstructionScript`)