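; BP_HUDHolder is an actor that hosts the 3D HUD widget for a VR minigame and exposes it to other gameplay code.
; On BeginPlay it casts its widget component's content to WBP_HUD3D and caches the reference.
; Wrapper functions check that reference is valid, then forward panel switching, countdown, score and game-over final score updates to the widget.
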(event `self.ReceiveBeginPlay`
  ; Initialises the HUDWidget
  (bind _aswbp_hud3d (cast `/Game/_CG_Projet_VR/MiniGame_Jonathan/HUD/Blueprints/WBP_HUD3D` (`WidgetComponent.GetWidget` (`self.Widget`))))
  (set `self.HUDWidgetRef` _aswbp_hud3d))

(fn `HUD_GameOver`
  (params (FinalScore :type Integer))
  (bind _hudwidgetref (`self.HUDWidgetRef`))
  ; Function that checks whether HUDWidget exists in order to update the final scores displayed on the HUD
  (`/Engine/EditorBlueprintResources/StandardMacros.IsValid` _hudwidgetref
    (:`Is Valid`
      (`/Game/_CG_Projet_VR/MiniGame_Jonathan/HUD/Blueprints/WBP_HUD3D.ShowGameOver` _hudwidgetref FinalScore))))

(fn `HUD_ShowPanel`
  (params (Panel :type "/Game/_CG_Projet_VR/MiniGame_Jonathan/HUD/E_HUDPanel Enum" :default "NewEnumerator0"))
  (bind _hudwidgetref (`self.HUDWidgetRef`))
  ; Function that checks whether HUDWidget exists in order to modify the HUD display panel
  (`/Engine/EditorBlueprintResources/StandardMacros.IsValid` _hudwidgetref
    (:`Is Valid`
      (`/Game/_CG_Projet_VR/MiniGame_Jonathan/HUD/Blueprints/WBP_HUD3D.ShowPanel` _hudwidgetref Panel))))

(fn `HUD_UpdateCountdown`
  (params (Value :type Integer))
  (bind _hudwidgetref (`self.HUDWidgetRef`))
  ; Function that checks whether HUDWidget exists Modify the HUD countdown
  (`/Engine/EditorBlueprintResources/StandardMacros.IsValid` _hudwidgetref
    (:`Is Valid`
      (`/Game/_CG_Projet_VR/MiniGame_Jonathan/HUD/Blueprints/WBP_HUD3D.UpdateCountdown` _hudwidgetref Value))))

(fn `HUD_UpdateScore`
  (params (Value :type "Float (double-precision)"))
  (bind _hudwidgetref (`self.HUDWidgetRef`))
  ; Function that checks whether HUDWidget exists in order to update the HUD score
  (`/Engine/EditorBlueprintResources/StandardMacros.IsValid` _hudwidgetref
    (:`Is Valid`
      (`/Game/_CG_Projet_VR/MiniGame_Jonathan/HUD/Blueprints/WBP_HUD3D.UpdateScore` _hudwidgetref Value))))

(fn `UserConstructionScript`)