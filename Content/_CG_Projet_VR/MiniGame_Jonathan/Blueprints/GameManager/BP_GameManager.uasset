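; Game manager for a VR mini-game where the player carries a ball on a tray while projectiles spawn.
; It binds start platform, HUD, spawner and ball events to a state machine: Idle, Countdown, Playing, GameOver.
; Playing attaches the tray to both motion controllers and runs timers that raise score and spawner difficulty.
; Ball death, projectile hits or leaving the platform request GameOver, intended to show results before resetting.
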(event `self.ReceiveBeginPlay`
  ; Initialising StartPlatform & Event binding
  (bind _outactors (`GameplayStatics.GetAllActorsOfClass` "/Game/_CG_Projet_VR/MiniGame_Jonathan/Blueprints/StartPlatform/BP_StartPlatform.BP_StartPlatform_C"))
  (bind _output (`|GetArrayItem` _outactors))
  (set `self.Ref_StartPlatform` _output)
  (add `/Game/_CG_Projet_VR/MiniGame_Jonathan/Blueprints/StartPlatform/BP_StartPlatform.OnPlayerEnterZone` _output (delegate `OnEnterZone_Handler`))
  (add `/Game/_CG_Projet_VR/MiniGame_Jonathan/Blueprints/StartPlatform/BP_StartPlatform.OnPlayerExitZone` (`self.Ref_StartPlatform`) (delegate `OnExitZone_Handler`))
  ; Initialising BP_HUDHolder & Event binding
  (bind _outactors_2 (`GameplayStatics.GetAllActorsOfClass` "/Game/_CG_Projet_VR/MiniGame_Jonathan/HUD/Blueprints/BP_HUDHolder.BP_HUDHolder_C"))
  (bind _output_2 (`|GetArrayItem` _outactors_2))
  (set `self.Ref_HUDHolder` _output_2)
  (bind _aswbp_hud3d (cast `/Game/_CG_Projet_VR/MiniGame_Jonathan/HUD/Blueprints/WBP_HUD3D` (`WidgetComponent.GetWidget` (`/Game/_CG_Projet_VR/MiniGame_Jonathan/HUD/Blueprints/BP_HUDHolder.Widget` _output_2))))
  (add `/Game/_CG_Projet_VR/MiniGame_Jonathan/HUD/Blueprints/WBP_HUD3D.OnPlayPressed` _aswbp_hud3d (delegate `OnPlayPressed_Handler`))
  (`/Game/_CG_Projet_VR/MiniGame_Jonathan/HUD/Blueprints/BP_HUDHolder.HUD_ShowPanel` (`self.Ref_HUDHolder`) "NewEnumerator0")
  ; Initialising BP_Tray
  (bind _outactors_3 (`GameplayStatics.GetAllActorsOfClass` "/Game/_CG_Projet_VR/MiniGame_Jonathan/Blueprints/Tray/BP_Tray.BP_Tray_C"))
  (set `self.Ref_Tray` (`|GetArrayItem` _outactors_3))
  ; Initialising BP_ProjectileSpawner & Event binding
  (bind _outactors_4 (`GameplayStatics.GetAllActorsOfClass` "/Game/_CG_Projet_VR/MiniGame_Jonathan/Blueprints/ProjectileSpawner/BP_ProjectileSpawner.BP_ProjectileSpawner_C"))
  (set `self.Ref_Spawner` (`|GetArrayItem` _outactors_4))
  (add `/Game/_CG_Projet_VR/MiniGame_Jonathan/Blueprints/ProjectileSpawner/BP_ProjectileSpawner.OnProjectileHitPlayer` (`self.Ref_Spawner`) (delegate `OnProjectileHit_Handler`))
  (`/Game/_CG_Projet_VR/MiniGame_Jonathan/HUD/Blueprints/BP_HUDHolder.HUD_ShowPanel` (`self.Ref_HUDHolder`) "NewEnumerator4"))

(event `OnProjectileHit_Handler`
  ; Event triggered when the pawn is hit by a projectile
  (if (`|EnumInequality` (`self.GameState`) "NewEnumerator3")
    (`self.SetGameState` "NewEnumerator3")))

(event `OnPlayPressed_Handler`
  ; Event triggered when the pawn interacts with the Play button on the HUD
  (if (`|EnumEquality` (`self.GameState`) "NewEnumerator0")
    (`self.SetGameState` "NewEnumerator1")))

(event `OnExitZone_Handler`
  ; An event that hides the HUDs when the player leaves the StartPlatform area and changes the game state
  (set `self.bPlayerInZone` false)
  (`/Game/_CG_Projet_VR/MiniGame_Jonathan/HUD/Blueprints/BP_HUDHolder.HUD_ShowPanel` (`self.Ref_HUDHolder`) "NewEnumerator4")
  (`KismetSystemLibrary.LogString` "Exit Zone")
  (if (`|EnumInequality` (`self.GameState`) "NewEnumerator3")
    (`self.SetGameState` "NewEnumerator3")))

(event `OnEnterZone_Handler`
  ; Event that displays the ‘Idle’ status HUD when entering the StartPlatform area
  (set `self.bPlayerInZone` true)
  (`KismetSystemLibrary.LogString` "Enter Zone")
  (if (`|EnumEquality` (`self.GameState`) "NewEnumerator0")
    (`/Game/_CG_Projet_VR/MiniGame_Jonathan/HUD/Blueprints/BP_HUDHolder.HUD_ShowPanel` (`self.Ref_HUDHolder`) "NewEnumerator0")))

(event `SetGameState`
  (params (NewState :type "/Game/_CG_Projet_VR/MiniGame_Jonathan/Blueprints/E_GameState Enum" :default "NewEnumerator0"))
  (bind _ref_tray (`self.Ref_Tray`))
  (bind _ref_tray_2 (`self.Ref_Tray`))
  (bind _ref_hudholder (`self.Ref_HUDHolder`))
  (bind _ref_hudholder_2 (`self.Ref_HUDHolder`))
  (bind _ref_hudholder_3 (`self.Ref_HUDHolder`))
  (bind _ref_tray_3 (`self.Ref_Tray`))
  (bind _ref_spawner (`self.Ref_Spawner`))
  (bind _ref_spawner_2 (`self.Ref_Spawner`))
  (switch `/Game/_CG_Projet_VR/MiniGame_Jonathan/Blueprints/E_GameState` NewState
    (:`NewEnumerator0`
      ; The player's status when they are ‘idle’
      (`KismetSystemLibrary.K2_ClearAndInvalidateTimerHandle` (`self.ScoreTimerHandle`))
      (`KismetSystemLibrary.K2_ClearAndInvalidateTimerHandle` (`self.DifficultyTimerHandle`))
      (`KismetSystemLibrary.K2_ClearAndInvalidateTimerHandle` (`self.CountdownTimerHandle`))
      (bind _outactors (`GameplayStatics.GetAllActorsOfClass` "/Game/_CG_Projet_VR/MiniGame_Jonathan/Blueprints/Ball/BP_Ball.BP_Ball_C"))
      (`self.K2_DestroyActor` _outactors)
      (`/Engine/EditorBlueprintResources/StandardMacros.IsValid` _ref_tray
        (:`Is Valid`
          (`/Game/_CG_Projet_VR/MiniGame_Jonathan/Blueprints/Tray/BP_Tray.DetachTray` _ref_tray)
          (bind _outactors_2 (`GameplayStatics.GetAllActorsOfClass` "/Game/_CG_Projet_VR/MiniGame_Jonathan/Blueprints/Ball/BP_Ball.BP_Ball_C"))
          (for _array_element _outactors_2
            (`self.K2_DestroyActor` _array_element)
            (`/Engine/EditorBlueprintResources/StandardMacros.IsValid` _ref_spawner
              (:`Is Valid`
                (`/Game/_CG_Projet_VR/MiniGame_Jonathan/Blueprints/ProjectileSpawner/BP_ProjectileSpawner.StopSpawning` _ref_spawner)
                (`/Engine/EditorBlueprintResources/StandardMacros.IsValid` _ref_tray_2
                  (:`Is Valid`
                    (`/Game/_CG_Projet_VR/MiniGame_Jonathan/Blueprints/Tray/BP_Tray.DetachTray` _ref_tray_2)
                    (set `self.CurrentScore` 0.0)
                    (set `self.CurrentDifficulty` 1)
                    (set `self.GameState` "NewEnumerator0")
                    (if (`self.bPlayerInZone`)
                      (`/Game/_CG_Projet_VR/MiniGame_Jonathan/HUD/Blueprints/BP_HUDHolder.HUD_ShowPanel` _ref_hudholder "NewEnumerator0")
                      (else
                        (`/Game/_CG_Projet_VR/MiniGame_Jonathan/HUD/Blueprints/BP_HUDHolder.HUD_ShowPanel` _ref_hudholder "NewEnumerator4")))))))))))
    (:`NewEnumerator1`
      ; The player's status when they are ‘Countdown’
      (set `self.GameState` "NewEnumerator1")
      (bind _output_get (set `self.CountdownValue` 5))
      (`/Game/_CG_Projet_VR/MiniGame_Jonathan/HUD/Blueprints/BP_HUDHolder.HUD_ShowPanel` (`self.Ref_HUDHolder`) "NewEnumerator1")
      (`/Game/_CG_Projet_VR/MiniGame_Jonathan/HUD/Blueprints/BP_HUDHolder.HUD_ShowPanel` _ref_hudholder_2 "NewEnumerator1")
      (`/Game/_CG_Projet_VR/MiniGame_Jonathan/HUD/Blueprints/BP_HUDHolder.HUD_UpdateCountdown` _ref_hudholder_2 _output_get)
      (`KismetSystemLibrary.K2_SetTimerDelegate` (delegate `TickCountdown`) 1.0 true))
    (:`NewEnumerator2`
      ; The player's status when they are ‘Playing’
      (set `self.GameState` "NewEnumerator2")
      (bind _asjh_vrpawn (cast `/Game/_CG_Projet_VR/MiniGame_Jacqueline/Blueprints/JH_VRPawn` (`GameplayStatics.GetPlayerPawn` 0)))
      (`/Game/_CG_Projet_VR/MiniGame_Jonathan/Blueprints/Tray/BP_Tray.AttachTray` (`self.Ref_Tray`) (`/Game/_CG_Projet_VR/MiniGame_Jacqueline/Blueprints/JH_VRPawn.MotionControllerLeftGrip` _asjh_vrpawn) (`/Game/_CG_Projet_VR/MiniGame_Jacqueline/Blueprints/JH_VRPawn.MotionControllerRightGrip` _asjh_vrpawn))
      (bind _returnvalue (`|SpawnActorFromClass` "/Game/_CG_Projet_VR/MiniGame_Jonathan/Blueprints/Ball/BP_Ball.BP_Ball_C" (`KismetMathLibrary.MakeTransform` (+ (`SceneComponent.K2_GetComponentLocation` (`/Game/_CG_Projet_VR/MiniGame_Jonathan/Blueprints/Tray/BP_Tray.TrayRoot` (`self.Ref_Tray`))) (0.0 0.0 25.0))) "Undefined" "MultiplyWithRoot" null null))
      (bind _output_get_2 (set `self.Ref_Ball` _returnvalue))
      (set `/Game/_CG_Projet_VR/MiniGame_Jonathan/Blueprints/Ball/BP_Ball.Ref_Tray` (`self.Ref_Tray`) _output_get_2)
      (add `/Game/_CG_Projet_VR/MiniGame_Jonathan/Blueprints/Ball/BP_Ball.OnBallDead` _output_get_2 (delegate `OnBallDead_Handler`))
      (`/Game/_CG_Projet_VR/MiniGame_Jonathan/Blueprints/ProjectileSpawner/BP_ProjectileSpawner.StartSpawning` (`self.Ref_Spawner`))
      (`/Game/_CG_Projet_VR/MiniGame_Jonathan/HUD/Blueprints/BP_HUDHolder.HUD_ShowPanel` _ref_hudholder_3 "NewEnumerator2")
      (`/Game/_CG_Projet_VR/MiniGame_Jonathan/HUD/Blueprints/BP_HUDHolder.HUD_UpdateScore` _ref_hudholder_3 0.0)
      (bind _returnvalue_2 (`KismetSystemLibrary.K2_SetTimer` null (`self.TickScoreFunction`) 0.1 true))
      (set `self.ScoreTimerHandle` _returnvalue_2)
      (bind _returnvalue_3 (`KismetSystemLibrary.K2_SetTimer` null (`self.TickDifficultyFunction`) 15.0 true))
      (set `self.DifficultyTimerHandle` _returnvalue_3))
    (:`NewEnumerator3`
      ; The player's status when they are ‘GameOver’
      (if (not (`|EnumInequality` (`self.GameState`) "NewEnumerator3"))
        (set `self.GameState` "NewEnumerator3")
        (`KismetSystemLibrary.K2_ClearAndInvalidateTimerHandle` (`self.ScoreTimerHandle`))
        (`KismetSystemLibrary.K2_ClearAndInvalidateTimerHandle` (`self.DifficultyTimerHandle`))
        (`KismetSystemLibrary.K2_ClearAndInvalidateTimerHandle` (`self.CountdownTimerHandle`))
        (`/Engine/EditorBlueprintResources/StandardMacros.IsValid` _ref_spawner_2
          (:`Is Valid`
            (`/Game/_CG_Projet_VR/MiniGame_Jonathan/Blueprints/ProjectileSpawner/BP_ProjectileSpawner.StopSpawning` _ref_spawner_2)
            (`/Engine/EditorBlueprintResources/StandardMacros.IsValid` _ref_tray_3
              (:`Is Valid`
                (`/Game/_CG_Projet_VR/MiniGame_Jonathan/Blueprints/Tray/BP_Tray.DetachTray` _ref_tray_3)
                (bind _outactors_3 (`GameplayStatics.GetAllActorsOfClass` "/Game/_CG_Projet_VR/MiniGame_Jonathan/Blueprints/Ball/BP_Ball.BP_Ball_C"))
                (for _array_element_2 _outactors_3
                  (`self.K2_DestroyActor` _array_element_2))
                (`/Game/_CG_Projet_VR/MiniGame_Jonathan/HUD/Blueprints/BP_HUDHolder.HUD_GameOver` (`self.Ref_HUDHolder`) (+ (`KismetMathLibrary.Round` (* (`self.CurrentScore`) 10.0)) (* (`self.CurrentDifficulty`) 50)))
                (`KismetSystemLibrary.Delay` 5.0)
                (`self.SetGameState` "NewEnumerator0")))))))))

(event `TickCountdown`
  (bind _countdownvalue (`self.CountdownValue`))
  ; An event that decrements the time for the countdown before the game begins
  (set `self.CountdownValue` (- _countdownvalue 1))
  (if (>= 0 _countdownvalue)
    (`KismetSystemLibrary.K2_ClearAndInvalidateTimerHandle` (`self.CountdownTimerHandle`))
    (`/Game/_CG_Projet_VR/MiniGame_Jonathan/HUD/Blueprints/BP_HUDHolder.HUD_UpdateCountdown` (`self.Ref_HUDHolder`) 0)
    (`KismetSystemLibrary.Delay` 0.8)
    (`self.SetGameState` "NewEnumerator2")
    (else
      (`/Game/_CG_Projet_VR/MiniGame_Jonathan/HUD/Blueprints/BP_HUDHolder.HUD_UpdateCountdown` (`self.Ref_HUDHolder`) (`self.CountdownValue`)))))

(event `OnBallDead_Handler`
  ; The player's status when they are ‘Playing’
  (if (`|EnumInequality` (`self.GameState`) "NewEnumerator3")
    (`self.SetGameState` "NewEnumerator3")))

(fn `TickDifficulty`
  (bind _output_get (set `self.CurrentDifficulty` (`KismetMathLibrary.Clamp` (+ (`self.CurrentDifficulty`) 1) 1 6)))
  (`/Engine/EditorBlueprintResources/StandardMacros.IsValid` (`self.Ref_Spawner`)
    (:`Is Valid`
      (`/Game/_CG_Projet_VR/MiniGame_Jonathan/Blueprints/ProjectileSpawner/BP_ProjectileSpawner.OnDifficultyUp` (`self.Ref_Spawner`) _output_get))))

(fn `TickScore`
  (bind _output_get (set `self.CurrentScore` (+ (`self.CurrentScore`) 0.1)))
  (`/Game/_CG_Projet_VR/MiniGame_Jonathan/HUD/Blueprints/BP_HUDHolder.HUD_UpdateScore` (`self.Ref_HUDHolder`) _output_get))

(fn `UserConstructionScript`)