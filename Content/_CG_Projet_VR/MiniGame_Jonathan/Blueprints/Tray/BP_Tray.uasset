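; VR minigame tray actor that is meant to be carried between two motion controllers.
; AttachTray saves the origin transform, centers the tray and starts a looping timer; DetachTray clears it and restores the transform.
; UpdateTrayTilt recenters the tray and smooths clamped roll and yaw from hand offsets.
; As written, the timer names UpdateTrayTiltFunction rather than UpdateTrayTilt, which also exits while IsAttached is true.
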(event `AttachTray`
  (params (MCLeft :type "MotionControllerComponent Object Reference") (MCRight :type "MotionControllerComponent Object Reference"))
  (set `self.Ref_MCLeft` MCLeft)
  (set `self.Ref_MCRight` MCRight)
  (set `self.OriginTransform` (`self.GetTransform`))
  (set `self.bIsAttached` true)
  (`self.K2_SetActorLocation` (/ (+ (`SceneComponent.K2_GetComponentLocation` (`self.Ref_MCLeft`)) (`SceneComponent.K2_GetComponentLocation` (`self.Ref_MCRight`))) 2.0))
  (bind _returnvalue (`KismetSystemLibrary.K2_SetTimer` null (`self.UpdateTrayTiltFunction`) 0.0 true))
  (set `self.TrayUpdateTimerHandle` _returnvalue))

(event `DetachTray`
  (`KismetSystemLibrary.K2_ClearAndInvalidateTimerHandle` (`self.TrayUpdateTimerHandle`))
  (set `self.bIsAttached` false)
  (`self.K2_SetActorTransform` (`self.OriginTransform`)))

(fn `UpdateTrayTilt`
  (bind _ref_mcleft (`self.Ref_MCLeft`))
  (bind _ref_mcright (`self.Ref_MCRight`))
  (bind _trayroot (`self.TrayRoot`))
  (bind _returnvalue (`SceneComponent.K2_GetComponentLocation` _ref_mcright))
  (bind _returnvalue_2 (`SceneComponent.K2_GetComponentLocation` _ref_mcleft))
  (bind _z (.z (- _returnvalue _returnvalue_2)))
  (if (`self.bIsAttached`)
    (return)
    (elif (`KismetSystemLibrary.IsValid` _ref_mcleft)
      (if (`KismetSystemLibrary.IsValid` _ref_mcright)
        (`self.K2_SetActorLocation` (/ (+ _returnvalue _returnvalue_2) 2.0))
        (`SceneComponent.K2_SetWorldRotation` _trayroot (`KismetMathLibrary.RLerp` (`SceneComponent.K2_GetComponentRotation` _trayroot) (`KismetMathLibrary.MakeRotator` (`KismetMathLibrary.FClamp` (`KismetMathLibrary.DegAtan2` _z (.y (- _returnvalue _returnvalue_2))) 35.0 15.0) 0.0 (`KismetMathLibrary.FClamp` (`KismetMathLibrary.DegAtan2` _z (.x (- _returnvalue _returnvalue_2))) -30.0 30.0)) 0.15 true) false false)
        (else
          (return)))
      (else
        (return)))))

(fn `UserConstructionScript`)