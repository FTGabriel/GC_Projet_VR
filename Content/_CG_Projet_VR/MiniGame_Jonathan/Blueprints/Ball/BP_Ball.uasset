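; BP_Ball is a physics-simulated ball for a VR minigame that detects when it falls below its tray.
; BeginPlay starts a looping timer meant to poll CheckFallZ, which compares ball height against the tray box plus an offset.
; On a fall, it clears the timer, disables collision and fires OnBallDead, though IsDead is set false rather than true.
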(event `self.ReceiveBeginPlay`
  (`PrimitiveComponent.SetSimulatePhysics` (`self.SM_Ball`) true)
  (bind _returnvalue (`KismetSystemLibrary.K2_SetTimer` null (`self.CheckFallZFunction`) 0.1 true))
  (set `self.FallCheckTimerHandle` _returnvalue))

(fn `CheckFallZ`
  (bind _ref_tray (`self.Ref_Tray`))
  (if (`self.bIsDead`)
    (return)
    (else
      (`/Engine/EditorBlueprintResources/StandardMacros.IsValid` _ref_tray
        (:`Is Valid`
          (if (> (+ (.z (`SceneComponent.K2_GetComponentLocation` (`/Game/_CG_Projet_VR/MiniGame_Jonathan/Blueprints/Tray/BP_Tray.TrayBox` _ref_tray))) (`self.FallThresholdOffset`)) (.z (`SceneComponent.K2_GetComponentLocation` (`self.SM_Ball`))))
            (set `self.bIsDead` false)
            (`KismetSystemLibrary.K2_ClearAndInvalidateTimerHandle` (`self.FallCheckTimerHandle`))
            (`PrimitiveComponent.SetCollisionEnabled` (`self.SM_Ball`) "NoCollision")
            (`self.OnBallDead`)
            (else
              (return))))))))

(fn `UserConstructionScript`)