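; Pooled projectile for a VR minigame that flies in a straight line and detects hits on the player pawn.
; Fire shows it, enables query collision and starts timers for fixed-step swept movement and a timed auto-return, avoiding Tick.
; Overlapping a JH_VRPawn returns it to the pool and broadcasts OnProjectileHitPlayer.
; ReturnToPool clears both timers, disables collision, hides the actor and parks it far below the world for reuse.
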(event `Fire`
  (params (Direction :type "Vector Structure") (InSpeed :type "Float (double-precision)"))
  (set `self.FireDirection` Direction)
  (set `self.Speed` InSpeed)
  (set `self.bHasHit` false)
  (`self.SetActorHiddenInGame` false)
  (`PrimitiveComponent.SetCollisionEnabled` (`self.ProjectileSphere`) "QueryOnly")
  (bind _returnvalue (`KismetSystemLibrary.K2_SetTimer` null (`self.MoveTickFunction`) 0.016 true))
  (set `self.MoveTimerHandle` _returnvalue)
  (bind _returnvalue_2 (`KismetSystemLibrary.K2_SetTimer` null (`self.ReturnToPoolFunction`) 3.0))
  (set `self.AutoReturnTimerHandle` _returnvalue_2))

(event `self.ProjectileSphere.OnComponentBeginOverlap`
  (params (OverlappedComponent :type "PrimitiveComponent Object Reference") (OtherActor :type "Actor Object Reference") (OtherComp :type "PrimitiveComponent Object Reference") (OtherBodyIndex :type Integer) (bFromSweep :type Boolean) (SweepResult :type "HitResult Structure (by ref)"))
  (if (not (`self.bHasHit`))
    (bind _asjh_vrpawn (cast `/Game/_CG_Projet_VR/MiniGame_Jacqueline/Blueprints/JH_VRPawn` (`ActorComponent.GetOwner` OtherComp)))
    (`/Engine/EditorBlueprintResources/StandardMacros.IsValid` _asjh_vrpawn
      (:`Is Valid`
        (set `self.bHasHit` true)
        (`self.ReturnToPool`)
        (`self.OnProjectileHitPlayer`)))))

(fn `MoveTick`
  (if (`self.bHasHit`)
    (return)
    (else
      (`self.K2_SetActorLocation` (+ (`self.K2_GetActorLocation`) (* (* (`self.FireDirection`) (`self.Speed`)) 0.016)) true))))

(fn `ReturnToPool`
  (`KismetSystemLibrary.K2_ClearAndInvalidateTimerHandle` (`self.MoveTimerHandle`))
  (`KismetSystemLibrary.K2_ClearAndInvalidateTimerHandle` (`self.AutoReturnTimerHandle`))
  (set `self.bHasHit` true)
  (`PrimitiveComponent.SetCollisionEnabled` (`self.ProjectileSphere`) "NoCollision")
  (`self.SetActorHiddenInGame` true)
  (`self.K2_SetActorLocation` (0.0 0.0 -10000.0)))

(fn `UserConstructionScript`)