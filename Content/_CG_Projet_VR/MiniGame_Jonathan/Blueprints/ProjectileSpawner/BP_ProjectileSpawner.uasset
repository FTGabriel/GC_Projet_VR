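; Spawner for a VR minigame that launches pooled projectiles toward the player pawn from random points around it.
; InitPool pre-spawns ten BP_Projectile actors far below the world and relays player hits through its own event.
; SpawnTick takes a hidden pool entry, places it using random spherical angles at SpawnRadius, then fires it.
; StartSpawning sets a looping timer, and StopSpawning clears it and returns every projectile to the pool.
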(event `self.ReceiveBeginPlay`
  (set `self.Ref_VRPawn` (`GameplayStatics.GetPlayerPawn` 0)))

(event `InitPool`
  (for _ (range 10)
    (bind _returnvalue (`|SpawnActorFromClass` "/Game/_CG_Projet_VR/MiniGame_Jonathan/Blueprints/Projectile/BP_Projectile.BP_Projectile_C" (`KismetMathLibrary.MakeTransform` (0.0 0.0 -10000.0)) "Undefined" "MultiplyWithRoot" null null))
    (`KismetArrayLibrary.Array_Add` (`self.ProjectilePool`) _returnvalue)
    (`self.SetActorHiddenInGame` false)
    (add `self.OnProjectileHitPlayer` (delegate `OnProjHit_Relay`))))

(event `OnProjHit_Relay`
  (`self.OnProjectileHitPlayer`))

(event `StartSpawning`
  (bind _returnvalue (`KismetSystemLibrary.K2_SetTimer` null (`self.SpawnTickFunction`) (`self.SpawnInterval`) true))
  (set `self.SpawnTimerHandle` _returnvalue))

(event `StopSpawning`
  (`KismetSystemLibrary.K2_ClearAndInvalidateTimerHandle` (`self.SpawnTimerHandle`))
  (for _array_element (`self.ProjectilePool`)
    (`/Game/_CG_Projet_VR/MiniGame_Jonathan/Blueprints/Projectile/BP_Projectile.ReturnToPool` _array_element)))

(fn `GetFromPool`
  (returns (FoundProjectile :type "/Game/_CG_Projet_VR/MiniGame_Jonathan/Blueprints/Projectile/BP_Projectile Object Reference"))
  (for _array_element (`self.ProjectilePool`)
    (if (`Actor.bHidden` _array_element)
      (return _array_element))))

(fn `SpawnTick`
  (bind _returnvalue (`KismetMathLibrary.RandomFloatInRange` -30.0 60.0))
  (bind _returnvalue_2 (`KismetMathLibrary.RandomFloatInRange` 0.0 360.0))
  (bind _spawnradius (`self.SpawnRadius`))
  (bind _returnvalue_3 (`KismetMathLibrary.DegCos` _returnvalue))
  (bind _returnvalue_4 (`SceneComponent.K2_GetComponentLocation` (`Actor.RootComponent` (`self.Ref_VRPawn`))))
  (bind _returnvalue_5 (+ _returnvalue_4 (`KismetMathLibrary.MakeVector` (* (`KismetMathLibrary.DegCos` _returnvalue_2) _returnvalue_3 _spawnradius) (* _spawnradius (`KismetMathLibrary.DegSin` _returnvalue_2) _returnvalue_3) (* _spawnradius (`KismetMathLibrary.DegSin` _returnvalue)))))
  (bind _foundprojectile (`self.GetFromPool`))
  (if (`KismetSystemLibrary.IsValid` _foundprojectile)
    (`self.K2_SetActorLocation` _foundprojectile _returnvalue_5 false false)
    (`self.SetActorHiddenInGame` _foundprojectile false)
    (`/Game/_CG_Projet_VR/MiniGame_Jonathan/Blueprints/Projectile/BP_Projectile.Fire` _foundprojectile (`KismetMathLibrary.Normal` (- _returnvalue_4 _returnvalue_5)) 0.0)
    (else
      (return))))

(fn `UserConstructionScript`)