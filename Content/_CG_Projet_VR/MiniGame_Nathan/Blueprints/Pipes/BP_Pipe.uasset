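; BP_Pipe is a colored pipe in a VR minigame that accepts bottles of the matching color.
; On overlap, it checks whether the bottle's material name contains the pipe's ColorName.
; A match plays a sound, flashes the pipe through a dynamic material's Intensity, fires haptics on both hands and destroys the bottle.
; As wired, AddScore runs only when the BP_ScoreDisplay lookup is invalid, so scoring looks inverted.
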(event `self.ReceiveBeginPlay`
  ; Change material at launch
  (`PrimitiveComponent.SetMaterial` (`self.Mesh_Pipe`) 0 (`self.Color Material`)))

(event `self.Collider.OnComponentBeginOverlap`
  (params (OverlappedComponent :type "PrimitiveComponent Object Reference") (OtherActor :type "Actor Object Reference") (OtherComp :type "PrimitiveComponent Object Reference") (OtherBodyIndex :type Integer) (bFromSweep :type Boolean) (SweepResult :type "HitResult Structure (by ref)"))
  (bind _returnvalue (`GameplayStatics.GetPlayerController` 0))
  (bind _mesh_pipe (`self.Mesh_Pipe`))
  ; Check if bottle entered pipe
  (bind _asbp_bottle (cast `/Game/_CG_Projet_VR/MiniGame_Nathan/Blueprints/Bottles/BP_Bottle` OtherActor))
  (if (`KismetStringLibrary.Contains` (`KismetSystemLibrary.GetObjectName` (`PrimitiveComponent.GetMaterial` (`/Game/_CG_Projet_VR/MiniGame_Nathan/Blueprints/Bottles/BP_Bottle.SM_Wine_Bottle` _asbp_bottle) 0)) (`self.ColorName`) false true)
    (`GameplayStatics.PlaySoundAtLocation` "/Engine/EditorSounds/Notifications/CompileSuccess.CompileSuccess" (`SceneComponent.K2_GetComponentLocation` (`self.Mesh_Pipe`)) (struct) 1.0 1.0 0.0 null null null null)
    (bind _returnvalue_2 (`PrimitiveComponent.CreateDynamicMaterialInstance` _mesh_pipe 0 (`PrimitiveComponent.GetMaterial` _mesh_pipe 0) "None"))
    (`MaterialInstanceDynamic.SetScalarParameterValue` _returnvalue_2 "Intensity" 10.0)
    (`KismetSystemLibrary.Delay` 0.2)
    (`MaterialInstanceDynamic.SetScalarParameterValue` _returnvalue_2 "Intensity" 0.0)
    (bind _returnvalue_3 (`GameplayStatics.GetActorOfClass` "/Game/_CG_Projet_VR/MiniGame_Nathan/Blueprints/Tools/BP_ScoreDisplay.BP_ScoreDisplay_C"))
    (`/Engine/EditorBlueprintResources/StandardMacros.IsValid` _returnvalue_3
      (:`Is Valid`
        _)
      (:`Is Not Valid`
        (`/Game/_CG_Projet_VR/MiniGame_Nathan/Blueprints/Tools/BP_ScoreDisplay.AddScore` _returnvalue_3 1.0)))
    (`KismetSystemLibrary.Delay` 0.5)
    (`PlayerController.PlayHapticEffect` _returnvalue "/Game/VRTemplate/Haptics/PistolFireHapticEffect.PistolFireHapticEffect" "Left" 1.0 false)
    (`PlayerController.PlayHapticEffect` _returnvalue "/Game/VRTemplate/Haptics/PistolFireHapticEffect.PistolFireHapticEffect" "Right" 1.0 false)
    (`self.K2_DestroyActor` _asbp_bottle)))

(fn `UserConstructionScript`)