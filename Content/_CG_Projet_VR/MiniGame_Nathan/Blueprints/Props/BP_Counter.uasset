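; BP_Counter is a Nathan minigame prop that starts rotation when the player steps into the middle of the counter.
; Overlapping the PlayerPosition trigger with a VRPawn or Character launches both its own BPRotationManager and the BP_RotationManager component on BP_Scene.
; Leaving the trigger stops both managers.
; Two DoOnce gates reset each other, so start and stop alternate without repeating.
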(event `self.PlayerPosition.OnComponentBeginOverlap`
  (params (OverlappedComponent :type "PrimitiveComponent Object Reference") (OtherActor :type "Actor Object Reference") (OtherComp :type "PrimitiveComponent Object Reference") (OtherBodyIndex :type Integer) (bFromSweep :type Boolean) (SweepResult :type "HitResult Structure (by ref)"))
  ; Start rotating when player go in middle of counter
  (cast `/Game/VRTemplate/Blueprints/VRPawn` OtherActor
    (:`then`
      _)
    (:`CastFailed`
      (cast `Character` OtherActor)))
  (`/Engine/EditorBlueprintResources/StandardMacros.DoOnce` false :!label _label
    (:`Completed`
      (`/Game/_CG_Projet_VR/MiniGame_Nathan/Blueprints/Tools/BP_RotationManager.Launch` (`self.BP_RotationManager`))
      (bind _returnvalue (`GameplayStatics.GetActorOfClass` "/Game/_CG_Projet_VR/MiniGame_Nathan/Blueprints/Props/BP_Scene.BP_Scene_C"))
      (`/Game/_CG_Projet_VR/MiniGame_Nathan/Blueprints/Tools/BP_RotationManager.Launch` (`self.GetComponentByClass` _returnvalue "/Game/_CG_Projet_VR/MiniGame_Nathan/Blueprints/Tools/BP_RotationManager.BP_RotationManager_C"))
      (goto _label_2 :!via `Reset`))))

(event `self.PlayerPosition.OnComponentEndOverlap`
  (params (OverlappedComponent :type "PrimitiveComponent Object Reference") (OtherActor :type "Actor Object Reference") (OtherComp :type "PrimitiveComponent Object Reference") (OtherBodyIndex :type Integer))
  ; Reset game
  (cast `/Game/VRTemplate/Blueprints/VRPawn` OtherActor
    (:`then`
      _)
    (:`CastFailed`
      (cast `Character` OtherActor)))
  (`/Engine/EditorBlueprintResources/StandardMacros.DoOnce` false :!label _label_2
    (:`Completed`
      (`/Game/_CG_Projet_VR/MiniGame_Nathan/Blueprints/Tools/BP_RotationManager.StopRotating` (`self.BP_RotationManager`))
      (bind _returnvalue (`GameplayStatics.GetActorOfClass` "/Game/_CG_Projet_VR/MiniGame_Nathan/Blueprints/Props/BP_Scene.BP_Scene_C"))
      (`/Game/_CG_Projet_VR/MiniGame_Nathan/Blueprints/Tools/BP_RotationManager.StopRotating` (`self.GetComponentByClass` _returnvalue "/Game/_CG_Projet_VR/MiniGame_Nathan/Blueprints/Tools/BP_RotationManager.BP_RotationManager_C"))
      (goto _label :!via `Reset`))))

(fn `UserConstructionScript`)