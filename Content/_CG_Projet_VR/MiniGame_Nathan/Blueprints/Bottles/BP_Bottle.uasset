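; BP_Bottle is a grabbable wine bottle for a VR mini-game, tinted with its ColorMaterial at BeginPlay.
; Grabbing it through GrabComponent, or calling Activate, detaches it in world space, enables physics and gravity, and switches collision to query-only.
; Dropping it, or calling Deactivate, turns physics and gravity off but leaves collision as query-only.
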(event `self.ReceiveBeginPlay`
  ; Change material at launch
  (`PrimitiveComponent.SetMaterial` (`self.SM_Wine_Bottle`) 0 (`self.ColorMaterial`)))

(event `self.GrabComponent.OnGrabbed`
  (bind _sm_wine_bottle (`self.SM_Wine_Bottle`))
  ; When grab bottle
  (`self.K2_DetachFromActor` "KeepWorld" "KeepWorld" "KeepWorld" :!label _label)
  (`PrimitiveComponent.SetSimulatePhysics` _sm_wine_bottle true)
  (`PrimitiveComponent.SetEnableGravity` _sm_wine_bottle true)
  (`PrimitiveComponent.SetCollisionEnabled` _sm_wine_bottle "QueryOnly"))

(event `Activate`
  ; When grab bottle
  (goto _label))

(event `self.GrabComponent.OnDropped`
  (bind _sm_wine_bottle (`self.SM_Wine_Bottle`))
  ; When release bottle
  (`PrimitiveComponent.SetSimulatePhysics` _sm_wine_bottle false :!label _label_2)
  (`PrimitiveComponent.SetEnableGravity` _sm_wine_bottle false))

(event `Deactivate`
  ; When release bottle
  (goto _label_2))

(fn `UserConstructionScript`)