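; BP_Spawner is a VR minigame tool that keeps a spawn point stocked with an object class, with special handling for bottles.
; It spawns CurrentObject at SpawnArrow on BeginPlay; BP_Bottle instances are deactivated and their mesh is snapped to the arrow.
; When an actor of that exact class leaves DetectZone, a replacement spawns after SpawnDelay.
; A DoOnce, reset after spawning, blocks overlapping respawn requests.
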(event `self.ReceiveBeginPlay`
  ; Spawn object at launch
  (`self.SpawnObject`))

(event `self.Detect Zone.OnComponentEndOverlap`
  (params (OverlappedComponent :type "PrimitiveComponent Object Reference") (OtherActor :type "Actor Object Reference") (OtherComp :type "PrimitiveComponent Object Reference") (OtherBodyIndex :type Integer))
  ; Respawn another object if previous exit detect zone
  (if (== (`GameplayStatics.GetObjectClass` OtherActor) (`self.CurrentObject`))
    (`/Engine/EditorBlueprintResources/StandardMacros.DoOnce` false :!label _label
      (:`Completed`
        (`KismetSystemLibrary.Delay` (`self.SpawnDelay`))
        (`self.SpawnObject`)
        (goto _label :!via `Reset`)))))

(fn `SpawnObject`
  (bind _currentobject (`self.CurrentObject`))
  (if (`KismetSystemLibrary.IsValidClass` _currentobject)
    (bind _returnvalue (`|SpawnActorFromClass` _currentobject (`SceneComponent.K2_GetComponentToWorld` (`self.SpawnArrow`)) "Undefined" "MultiplyWithRoot" null null))
    (set `self.CurrentObject` (`GameplayStatics.GetObjectClass` _returnvalue))
    (bind _asbp_bottle (cast `/Game/_CG_Projet_VR/MiniGame_Nathan/Blueprints/Bottles/BP_Bottle` _returnvalue))
    (`/Game/_CG_Projet_VR/MiniGame_Nathan/Blueprints/Bottles/BP_Bottle.Deactivate` _asbp_bottle)
    (`SceneComponent.K2_AttachToComponent` (`/Game/_CG_Projet_VR/MiniGame_Nathan/Blueprints/Bottles/BP_Bottle.SM_Wine_Bottle` _asbp_bottle) (`self.SpawnArrow`) "None" "SnapToTarget" "SnapToTarget" "KeepWorld" true)))

(fn `UserConstructionScript`)