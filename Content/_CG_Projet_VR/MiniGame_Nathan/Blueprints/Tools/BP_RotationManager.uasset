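; Actor component that makes its owner spin progressively faster over time, apparently for a rotating counter in a VR minigame.
; On BeginPlay it caches the owner's first RotatingMovementComponent and zeroes its rotation rate.
; A looping timer then raises the speed by a fixed increment up to a maximum, scales it by the configured axis and applies it as the new rotation rate.
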(event `self.ReceiveBeginPlay`
  (bind _output (`|GetArrayItem` (`Actor.K2_GetComponentsByClass` (`self.GetOwner`) "/Script/Engine.RotatingMovementComponent")))
  ; Start event and make counter static
  (`KismetSystemLibrary.K2_SetTimerDelegate` (delegate `IncreaseSpeed`) (`self.SpeedDelay`) true)
  (`/Engine/EditorBlueprintResources/StandardMacros.IsValid` _output
    (:`Is Valid`
      (bind _output_get (set `self.RotatingComponent` _output))
      (set `RotatingMovementComponent.RotationRate` (struct) _output_get))))

(event `IncreaseSpeed`
  (bind _rotatingcomponent (`self.RotatingComponent`))
  (bind (_rotationaxis_roll _rotationaxis_pitch _rotationaxis_yaw) (`KismetMathLibrary.BreakRotator` (`self.RotationAxis`)))
  ; Make counter turn faster every minute
  (bind _output_get (set `self.Current Speed` (`KismetMathLibrary.FClamp` (+ (`self.Current Speed`) (`self.IncrementSpeed`)) 0.0 (`self.MaxSpeed`))))
  (`/Engine/EditorBlueprintResources/StandardMacros.IsValid` _rotatingcomponent
    (:`Is Valid`
      (set `RotatingMovementComponent.RotationRate` (`KismetMathLibrary.MakeRotator` (* _output_get _rotationaxis_roll) (* _output_get _rotationaxis_pitch) (* _output_get _rotationaxis_yaw)) _rotatingcomponent))))