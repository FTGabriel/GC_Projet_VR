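; BP_ScoreDisplay is a score display actor for the Nathan VR minigame that keeps and shows a running score.
; AddScore adds a given amount to the stored Score, then calls UpdateScore.
; UpdateScore casts the widget component's user widget to W_ScoreWidget and sets its ScoreText to the formatted score in points.
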(event `AddScore`
  (params (ScoreAmount :type "Float (double-precision)"))
  (set `self.Score` (+ ScoreAmount (`self.Score`)))
  (`self.UpdateScore`))

(event `UpdateScore`
  (bind _asw_score_widget (cast `/Game/_CG_Projet_VR/MiniGame_Nathan/Blueprints/Tools/W_ScoreWidget` (`WidgetComponent.GetUserWidgetObject` (`self.Widget`))))
  (`TextBlock.SetText` (`/Game/_CG_Projet_VR/MiniGame_Nathan/Blueprints/Tools/W_ScoreWidget.ScoreText` _asw_score_widget) (`|FormatText` "Score : {score} pts" (`self.Score`))))

(fn `UserConstructionScript`)