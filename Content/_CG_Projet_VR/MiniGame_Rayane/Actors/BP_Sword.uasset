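; BP_Sword is a sword actor for a VR minigame that destroys boxes whose color matches its sword type.
; On BeginPlay it caches the RB_VRPawn as Player.
; Its Box overlap filters for BPI_Destructible, casts to BP_MBox, and compares the mesh's blue or red material against SwordType.
; A match destroys the box and calls CallIncrease on the pawn, while mismatches are ignored.
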(event `self.ReceiveBeginPlay`
  (bind _returnvalue (`GameplayStatics.GetActorOfClass` "/Game/_CG_Projet_VR/MiniGame_Rayane/Actors/RB_VRPawn.RB_VRPawn_C"))
  (set `self.Player` _returnvalue))

(event `self.Box.OnComponentBeginOverlap`
  (params (OverlappedComponent :type "PrimitiveComponent Object Reference") (OtherActor :type "Actor Object Reference") (OtherComp :type "PrimitiveComponent Object Reference") (OtherBodyIndex :type Integer) (bFromSweep :type Boolean) (SweepResult :type "HitResult Structure (by ref)"))
  (if (`KismetSystemLibrary.DoesImplementInterface` OtherActor "/Game/_CG_Projet_VR/MiniGame_Rayane/Core/Interface/BPI_Destructible.BPI_Destructible_C")
    (bind _asbp_mbox (cast `/Game/_CG_Projet_VR/MiniGame_Rayane/Actors/BP_MBox` OtherActor))
    (bind _staticmesh (`/Game/_CG_Projet_VR/MiniGame_Rayane/Actors/BP_MBox.StaticMesh` _asbp_mbox))
    (if (and (== (`PrimitiveComponent.GetMaterial` _staticmesh 0) "/Game/_CG_Projet_VR/MiniGame_Rayane/Assets/Materials/MI_Box_Blue.MI_Box_Blue") (`|EnumEquality` (`self.SwordType`) "NewEnumerator0"))
      (`self.K2_DestroyActor` OtherActor)
      (`/Game/_CG_Projet_VR/MiniGame_Rayane/Actors/RB_VRPawn.CallIncrease` (`self.Player`) :!label _label)
      (elif (and (== (`PrimitiveComponent.GetMaterial` _staticmesh 0) "/Game/_CG_Projet_VR/MiniGame_Rayane/Assets/Materials/MI_Box_Red.MI_Box_Red") (`|EnumEquality` (`self.SwordType`) "NewEnumerator1"))
        (`self.K2_DestroyActor` OtherActor)
        (goto _label)))))

(fn `UserConstructionScript`)