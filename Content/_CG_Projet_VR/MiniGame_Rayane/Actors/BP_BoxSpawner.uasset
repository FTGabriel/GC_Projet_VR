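; BP_BoxSpawner drives a VR rhythm minigame, playing a song and spawning BP_MBox actors on its loud moments.
; BeginPlay starts the sound from the first loudness NRT asset and writes a hardcoded title into the WB_Score widget.
; Tick samples that asset's precomputed normalized loudness at game time, spawning above a threshold at a random left or right arrow.
; Colliding spawns are skipped, and each new box gets a random blue or red material.
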(event `self.ReceiveBeginPlay`
  (if (> (`KismetArrayLibrary.Array_Length` (`self.SongLoudnessNRTContainer`)) 0)
    (`GameplayStatics.PlaySound2D` (`AudioAnalyzerNRT.Sound` (`|GetArrayItem` (`self.SongLoudnessNRTContainer`))) 1.0 1.0 0.0 null null)
    (bind _aswb_score (cast `/Game/_CG_Projet_VR/MiniGame_Rayane/Core/Widgets/WB_Score` (`WidgetComponent.GetWidget` (`self.Widget`))))
    (`TextBlock.SetText` (`/Game/_CG_Projet_VR/MiniGame_Rayane/Core/Widgets/WB_Score.SongName` _aswb_score) "Rust On The Code")
    (else
      (`KismetSystemLibrary.PrintString` "NRTContainer is empty"))))

(event `self.ReceiveTick`
  (params (DeltaSeconds :type "Float (single-precision)"))
  (if (> (`LoudnessNRT.GetNormalizedLoudnessAtTime` (`|GetArrayItem` (`self.SongLoudnessNRTContainer`)) (`KismetSystemLibrary.GetGameTimeInSeconds`)) 0.7)
    (bind _returnvalue (`|SpawnActorFromClass` "/Game/_CG_Projet_VR/MiniGame_Rayane/Actors/BP_MBox.BP_MBox_C" (`KismetMathLibrary.SelectTransform` (`SceneComponent.K2_GetComponentToWorld` (`self.Arrow_Right2`)) (`SceneComponent.K2_GetComponentToWorld` (`self.Arrow_Left2`)) (`KismetMathLibrary.RandomBool`)) "DontSpawnIfColliding" "MultiplyWithRoot" null null))
    (`/Engine/EditorBlueprintResources/StandardMacros.IsValid` _returnvalue
      (:`Is Valid`
        (switch `int` (`KismetMathLibrary.RandomIntegerInRange` 0 1)
          (:`0`
            (bind _staticmesh (`/Game/_CG_Projet_VR/MiniGame_Rayane/Actors/BP_MBox.StaticMesh` _returnvalue))
            (`PrimitiveComponent.SetMaterial` _staticmesh 0 "/Game/_CG_Projet_VR/MiniGame_Rayane/Assets/Materials/MI_Box_Blue.MI_Box_Blue"))
          (:`1`
            (`PrimitiveComponent.SetMaterial` _staticmesh 0 "/Game/_CG_Projet_VR/MiniGame_Rayane/Assets/Materials/MI_Box_Red.MI_Box_Red")))))))

(fn `UserConstructionScript`)